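; Slate puzzle manager that completes a quest once all four referenced slates hold correct answers.
; On BeginPlay it binds a handler to each slate's answer-input event, which writes that slate's correctness into an indexed Answers array.
; Every input rechecks the whole array, printing Correct or Wrong for the combined result.
; When all are true, it calls quest completion and adds an alert through the player character's BPSystem.
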(event Custom|CheckUserAnswer1
  (CallFunction|GetSlatesAnswers (Variables|/Game/Items/Parents/BP_P_Slate.BP_P_Slate_C|GetIsUserAnswerCorrect (Variables|Default|GetSlate1))))

(event Custom|CheckUserAnswer2
  (CallFunction|GetSlatesAnswers (Variables|/Game/Items/Parents/BP_P_Slate.BP_P_Slate_C|GetIsUserAnswerCorrect (Variables|Default|GetSlate2)) 1))

(event Custom|CheckUserAnswer3
  (CallFunction|GetSlatesAnswers (Variables|/Game/Items/Parents/BP_P_Slate.BP_P_Slate_C|GetIsUserAnswerCorrect (Variables|Default|GetSlate3)) 2))

(event Custom|CheckUserAnswer4
  (CallFunction|GetSlatesAnswers (Variables|/Game/Items/Parents/BP_P_Slate.BP_P_Slate_C|GetIsUserAnswerCorrect (Variables|Default|GetSlate4)) 3))

(event EventBeginPlay
  (Utilities|FlowControl|Sequence
    (:then_0
      (EventDispatchers|BindEventtoOnUserAnswerInput (Variables|Default|GetSlate1) (delegate Custom|CheckUserAnswer1)))
    (:then_1
      (EventDispatchers|BindEventtoOnUserAnswerInput (Variables|Default|GetSlate2) (delegate Custom|CheckUserAnswer2)))
    (:then_2
      (EventDispatchers|BindEventtoOnUserAnswerInput (Variables|Default|GetSlate3) (delegate Custom|CheckUserAnswer3)))
    (:then_3
      (EventDispatchers|BindEventtoOnUserAnswerInput (Variables|Default|GetSlate4) (delegate Custom|CheckUserAnswer4)))))

(fn ConstructionScript)

(fn GetSlatesAnswers
  (params (SlateAnswer :type Boolean) (Index :type Integer))
  (Utilities|Array|SetArrayElem (Variables|Default|GetAnswers) Index SlateAnswer)
  (bind _newparam (CallFunction|CheckAnswers))
  (if _newparam
    (Development|PrintString "Correct!!!")
    (else
      (Development|PrintString "Wrong!!!"))))

(fn CheckAnswers
  (bind _answers (Variables|Default|GetAnswers))
  (bind _answers_2 (Variables|Default|GetAnswers))
  (bind _answers_3 (Variables|Default|GetAnswers))
  (bind _answers_4 (Variables|Default|GetAnswers))
  (bind _output (Utilities|Array|Get(acopy) _answers 3))
  (bind _output_2 (Utilities|Array|Get(acopy) _answers_2))
  (bind _output_3 (Utilities|Array|Get(acopy) _answers_3 1))
  (bind _output_4 (Utilities|Array|Get(acopy) _answers_4 2))
  (bind _returnvalue (Math|Boolean|ANDBoolean _output_2 _output_3 _output_4 _output))
  (bind _asbp_top_down_character (Utilities|Casting|CastToBP_TopDownCharacter (Game|GetPlayerCharacter 0)))
  (if _returnvalue
    (Default|QuestComplete (Variables|/Game/TopDown/Blueprints/BP_TopDownCharacter.BP_TopDownCharacter_C|GetBP_System _asbp_top_down_character) 10 "Quest")
    (Default|AlertAdd (Variables|/Game/TopDown/Blueprints/BP_TopDownCharacter.BP_TopDownCharacter_C|GetBP_System _asbp_top_down_character) 9)
    (return _returnvalue)
    (else
      (return _returnvalue))))