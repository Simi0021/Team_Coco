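; BP_Slate4 is a puzzle slate, a child Blueprint that sets its Answer to 4 on BeginPlay after calling the parent.
; When BP_TopDownCharacter overlaps its capsule, it plays the Fa note as a 2D sound unless IsAllAnswerCorrect is already true.
; It contains no answer-checking logic of its own, and its Tick and actor-overlap events are disabled.
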(event OnComponentBeginOverlap(Capsule)
  (params (OverlappedComponent :type Primitive%20Component%20Object%20Reference) (OtherActor :type Actor%20Object%20Reference) (OtherComp :type Primitive%20Component%20Object%20Reference) (OtherBodyIndex :type Integer) (bFromSweep :type Boolean) (SweepResult :type Hit%20Result%20Structure%20%28by%20ref%29))
  (Utilities|Casting|CastToBP_TopDownCharacter OtherActor)
  (if (not (Variables|Default|GetIsAllAnswerCorrect))
    (Audio|PlaySound2D "/Game/Sounds/Fa.Fa" 1.0 1.0 0.0 0 0)))

(event EventBeginPlay
  (|CallParentFunction)
  (Variables|Default|SetAnswer 4))

(event Collision|EventActorBeginOverlap
  (params (OtherActor :type Actor%20Object%20Reference))
  (|CallParentFunction OtherActor) ; This node is disabled and will not be called.\nDrag off pins to build functionality.
)

(event EventTick
  (params (DeltaSeconds :type Float%20%28single-precision%29))
  (|CallParentFunction DeltaSeconds) ; This node is disabled and will not be called.\nDrag off pins to build functionality.
)

(fn ConstructionScript
  (|CallParentFunction))