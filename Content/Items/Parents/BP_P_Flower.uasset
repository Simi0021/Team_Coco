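; BP_P_Flower is a flower interactable that exchanges one inventory item for another.
; Its capsule sets or clears itself as LookAtActor on the top-down character's inventory component as that character enters or leaves.
; On InteractionE it searches GI_SoulCatcher's InventoryContent for an exact ChangingItemID and Quantity match, empties that slot, then adds ItemToChange in the same quantity through the inventory component.
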(event OnComponentBeginOverlap(Capsule)
  (params (OverlappedComponent :type Primitive%20Component%20Object%20Reference) (OtherActor :type Actor%20Object%20Reference) (OtherComp :type Primitive%20Component%20Object%20Reference) (OtherBodyIndex :type Integer) (bFromSweep :type Boolean) (SweepResult :type Hit%20Result%20Structure%20%28by%20ref%29))
  (bind _asbp_top_down_character (Utilities|Casting|CastToBP_TopDownCharacter OtherActor))
  (Variables|/Game/TopDown/Blueprints/Inventory/BP_InventorySystem.BP_InventorySystem_C|SetLookAtActor (Variables|/Game/TopDown/Blueprints/BP_TopDownCharacter.BP_TopDownCharacter_C|GetBP_InventorySystem _asbp_top_down_character) self))

(event OnComponentEndOverlap(Capsule)
  (params (OverlappedComponent :type Primitive%20Component%20Object%20Reference) (OtherActor :type Actor%20Object%20Reference) (OtherComp :type Primitive%20Component%20Object%20Reference) (OtherBodyIndex :type Integer))
  (bind _asbp_top_down_character (Utilities|Casting|CastToBP_TopDownCharacter OtherActor))
  (Variables|/Game/TopDown/Blueprints/Inventory/BP_InventorySystem.BP_InventorySystem_C|SetLookAtActor (Variables|/Game/TopDown/Blueprints/BP_TopDownCharacter.BP_TopDownCharacter_C|GetBP_InventorySystem _asbp_top_down_character) 0))

(event EventBeginPlay)

(event Collision|EventActorBeginOverlap
  (params (OtherActor :type Actor%20Object%20Reference)))

(event EventTick
  (params (DeltaSeconds :type Float%20%28single-precision%29)))

(event EventInteractionE
  (bind _returnvalue (Game|GetPlayerCharacter 0))
  (bind _asbp_top_down_character (Utilities|Casting|CastToBP_TopDownCharacter _returnvalue))
  (bind _bp_inventorysystem (Variables|/Game/TopDown/Blueprints/BP_TopDownCharacter.BP_TopDownCharacter_C|GetBP_InventorySystem _asbp_top_down_character))
  (Utilities|IsValid _bp_inventorysystem
    (:Is%20Valid
      (bind _asgi_soul_catcher (Utilities|Casting|CastToGI_SoulCatcher (Game|GetGameInstance)))
      (if (Utilities|Array|ContainsItem (Variables|/Game/TopDown/Blueprints/SaveGame/GI_SoulCatcher.GI_SoulCatcher_C|GetInventory%20Content _asgi_soul_catcher) (Utilities|Struct|MakeF_InventorySlotStruct (Variables|Default|GetChangingItemID) (Variables|Default|GetQuantity)))
        (Utilities|Array|SetArrayElem (Variables|/Game/TopDown/Blueprints/SaveGame/GI_SoulCatcher.GI_SoulCatcher_C|GetInventory%20Content _asgi_soul_catcher) (Utilities|Array|FindItem (Variables|/Game/TopDown/Blueprints/SaveGame/GI_SoulCatcher.GI_SoulCatcher_C|GetInventory%20Content _asgi_soul_catcher) (Utilities|Struct|MakeF_InventorySlotStruct (Variables|Default|GetChangingItemID) (Variables|Default|GetQuantity))) (Utilities|Struct|MakeF_InventorySlotStruct "" 0))
        (Default|AddItemtoInventory _bp_inventorysystem (Variables|Default|GetItemToChange) (Variables|Default|GetQuantity))))))

(fn ConstructionScript)

(fn InRangeOf
  (return ""))