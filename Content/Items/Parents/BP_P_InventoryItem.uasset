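; BP_P_InventoryItem is a parent Blueprint for world items that prompts the top-down character to pick them up when in range.
; Capsule overlap sets the item as the LookAtActor on the character's inventory system and shows a message, then clears both on exit.
; InRangeOf builds the "Pick up {Item}" text from the name in the data table row referenced by the item data component's ItemID.
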(event OnComponentBeginOverlap(Capsule)
  (params (OverlappedComponent :type Primitive%20Component%20Object%20Reference) (OtherActor :type Actor%20Object%20Reference) (OtherComp :type Primitive%20Component%20Object%20Reference) (OtherBodyIndex :type Integer) (bFromSweep :type Boolean) (SweepResult :type Hit%20Result%20Structure%20%28by%20ref%29))
  (bind _asbp_top_down_character (Utilities|Casting|CastToBP_TopDownCharacter OtherActor))
  (Variables|/Game/TopDown/Blueprints/Inventory/BP_InventorySystem.BP_InventorySystem_C|SetLookAtActor (Variables|/Game/TopDown/Blueprints/BP_TopDownCharacter.BP_TopDownCharacter_C|GetBP_InventorySystem _asbp_top_down_character) self)
  (bind _message (CallFunction|InRangeOf))
  (Default|ShowMessage (Variables|/Game/TopDown/Blueprints/Inventory/BP_InventorySystem.BP_InventorySystem_C|GetDisplayMessageRef (Variables|/Game/TopDown/Blueprints/BP_TopDownCharacter.BP_TopDownCharacter_C|GetBP_InventorySystem _asbp_top_down_character)) _message))

(event OnComponentEndOverlap(Capsule)
  (params (OverlappedComponent :type Primitive%20Component%20Object%20Reference) (OtherActor :type Actor%20Object%20Reference) (OtherComp :type Primitive%20Component%20Object%20Reference) (OtherBodyIndex :type Integer))
  (bind _asbp_top_down_character (Utilities|Casting|CastToBP_TopDownCharacter OtherActor))
  (Variables|/Game/TopDown/Blueprints/Inventory/BP_InventorySystem.BP_InventorySystem_C|SetLookAtActor (Variables|/Game/TopDown/Blueprints/BP_TopDownCharacter.BP_TopDownCharacter_C|GetBP_InventorySystem _asbp_top_down_character) 0)
  (Default|ShowMessage (Variables|/Game/TopDown/Blueprints/Inventory/BP_InventorySystem.BP_InventorySystem_C|GetDisplayMessageRef (Variables|/Game/TopDown/Blueprints/BP_TopDownCharacter.BP_TopDownCharacter_C|GetBP_InventorySystem _asbp_top_down_character))))

(event EventBeginPlay)

(event Collision|EventActorBeginOverlap
  (params (OtherActor :type Actor%20Object%20Reference)))

(event EventTick
  (params (DeltaSeconds :type Float%20%28single-precision%29)))

(fn ConstructionScript)

(fn InRangeOf
  (bind _bp_itemdatacomponent (Variables|Default|GetBP_ItemDataComponent))
  (bind _itemid (Variables|/Game/TopDown/Blueprints/Inventory/BP_ItemDataComponent.BP_ItemDataComponent_C|GetItemID _bp_itemdatacomponent))
  (bind _returnvalue (Utilities|GetDataTableRow (.datatable _itemid) (.rowname _itemid))
    (:then
      (return (Utilities|Text|FormatText "Pick up {Item}" (.Name (Utilities|Struct|BreakF_ItemStruct _returnvalue)))))))