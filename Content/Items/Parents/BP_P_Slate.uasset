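; BP_P_Slate is a parent puzzle actor for slates that the player changes with inventory items and that check for a correct answer.
; Capsule overlap sets it as the player's LookAtActor, and interacting opens the slate menu until all answers are correct.
; Confirm maps the first game-instance inventory item to a material, swaps in an empty bottle, compares against Answer and fires OnUserAnswerInput.
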(event OnComponentBeginOverlap(Capsule)
  (params (OverlappedComponent :type Primitive%20Component%20Object%20Reference) (OtherActor :type Actor%20Object%20Reference) (OtherComp :type Primitive%20Component%20Object%20Reference) (OtherBodyIndex :type Integer) (bFromSweep :type Boolean) (SweepResult :type Hit%20Result%20Structure%20%28by%20ref%29))
  (bind _asbp_top_down_character (Utilities|Casting|CastToBP_TopDownCharacter OtherActor))
  (Variables|/Game/TopDown/Blueprints/Inventory/BP_InventorySystem.BP_InventorySystem_C|SetLookAtActor (Variables|/Game/TopDown/Blueprints/BP_TopDownCharacter.BP_TopDownCharacter_C|GetBP_InventorySystem _asbp_top_down_character) self))

(event OnComponentEndOverlap(Capsule)
  (params (OverlappedComponent :type Primitive%20Component%20Object%20Reference) (OtherActor :type Actor%20Object%20Reference) (OtherComp :type Primitive%20Component%20Object%20Reference) (OtherBodyIndex :type Integer))
  (bind _slatewidgetref (Variables|Default|GetSlateWidgetRef))
  (bind _asbp_top_down_character (Utilities|Casting|CastToBP_TopDownCharacter OtherActor))
  (Variables|/Game/TopDown/Blueprints/Inventory/BP_InventorySystem.BP_InventorySystem_C|SetLookAtActor (Variables|/Game/TopDown/Blueprints/BP_TopDownCharacter.BP_TopDownCharacter_C|GetBP_InventorySystem _asbp_top_down_character) 0)
  (Utilities|IsValid _slatewidgetref
    (:Is%20Valid
      (Widget|RemovefromParent _slatewidgetref))))

(event Custom|ChangeSlateMaterialBaseOnItem
  (bind _asgi_soul_catcher (Utilities|Casting|CastToGI_SoulCatcher (Game|GetGameInstance)))
  (switch name (.ItemID (Utilities|Struct|BreakF_InventorySlotStruct (Utilities|Array|Get(acopy) (Variables|/Game/TopDown/Blueprints/SaveGame/GI_SoulCatcher.GI_SoulCatcher_C|GetInventory%20Content _asgi_soul_catcher))))
    (:17
      (bind _iscorrectanswer (CallFunction|SlateInteraction))
      (Variables|Default|SetIsUserAnswerCorrect _iscorrectanswer)
      (Default|CallOnUserAnswerInput))
    (:18
      (bind _iscorrectanswer_2 (CallFunction|SlateInteraction 1))
      (Variables|Default|SetIsUserAnswerCorrect _iscorrectanswer_2)
      (Default|CallOnUserAnswerInput))
    (:19
      (bind _iscorrectanswer_3 (CallFunction|SlateInteraction 2))
      (Variables|Default|SetIsUserAnswerCorrect _iscorrectanswer_3)
      (Default|CallOnUserAnswerInput))
    (:20
      (bind _iscorrectanswer_4 (CallFunction|SlateInteraction 3))
      (Variables|Default|SetIsUserAnswerCorrect _iscorrectanswer_4)
      (Default|CallOnUserAnswerInput))))

(event Custom|RemoveWidget
  (Widget|RemovefromParent (Variables|Default|GetSlateWidgetRef)))

(event EventBeginPlay)

(event Collision|EventActorBeginOverlap
  (params (OtherActor :type Actor%20Object%20Reference)))

(event EventTick
  (params (DeltaSeconds :type Float%20%28single-precision%29)))

(event EventInteractwith
  (params (PlayerCharacter :type BP%20Top%20Down%20Character%20Object%20Reference))
  (if (not (Variables|Default|GetIsAllAnswerCorrect))
    (Default|InventoryOff (.AsBP%20Top%20Down%20Controller (Utilities|Casting|CastToBP_TopDownController (Game|GetPlayerController 0))))
    (Utilities|IsValid (Variables|Default|GetSlateWidgetRef)
      (:Is%20Valid
        _)
      (:Is%20Not%20Valid
        (bind _returnvalue (UserInterface|CreateWidget "/Game/TopDown/Blueprints/Inventory/UI/WBP_SlateMenu.WBP_SlateMenu_C" 0 (Variables|Default|GetBP_InventorySystem)))
        (Variables|Default|SetSlateWidgetRef _returnvalue)))
    (UserInterface|Viewport|AddtoViewport (Variables|Default|GetSlateWidgetRef) 0)
    (EventDispatchers|BindEventtoOnClicked (Variables|/Game/TopDown/Blueprints/Inventory/UI/WBP_SlateMenu.WBP_SlateMenu_C|GetBTN_Exit (Variables|Default|GetSlateWidgetRef)) (delegate Custom|RemoveWidget))
    (EventDispatchers|AssignOnClicked (Variables|/Game/TopDown/Blueprints/Inventory/UI/WBP_SlateMenu.WBP_SlateMenu_C|GetBTN_Confirm (Variables|Default|GetSlateWidgetRef)) (delegate Custom|ChangeSlateMaterialBaseOnItem))))

(fn ConstructionScript)

(fn ChangeMaterial
  (params (Index :type Integer))
  (Rendering|Material|SetMaterial (Variables|Default|GetStaticMesh) 0 (Utilities|Array|Get(acopy) (Variables|Default|GetChangingMaterial) Index)))

(fn ChangeItemtoEmptyBottle
  (params (Index :type Integer))
  (bind _asgi_soul_catcher (Utilities|Casting|CastToGI_SoulCatcher (Game|GetGameInstance)))
  (Utilities|Array|SetArrayElem (Variables|/Game/TopDown/Blueprints/SaveGame/GI_SoulCatcher.GI_SoulCatcher_C|GetInventory%20Content _asgi_soul_catcher) 0 (Utilities|Struct|MakeF_InventorySlotStruct "" 0))
  (Utilities|Array|SetArrayElem (Variables|/Game/TopDown/Blueprints/SaveGame/GI_SoulCatcher.GI_SoulCatcher_C|GetInventory%20Content _asgi_soul_catcher) 0 (Utilities|Struct|MakeF_InventorySlotStruct (Utilities|Array|Get(acopy) (LocalVariables|GetItemID) Index) 1))
  (Default|Update (Variables|Default|GetBP_InventorySystem)))

(fn SlateInteraction
  (params (Index :type Integer))
  (CallFunction|ChangeMaterial Index)
  (CallFunction|ChangeItemtoEmptyBottle Index)
  (return (== (Variables|Default|GetAnswer) (+ Index 1))))

(fn InRangeOf
  (return ""))