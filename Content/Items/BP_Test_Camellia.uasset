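; BP_Test_Camellia is an interactable pickup item, apparently a test asset tied to the Old Man NPC's quest.
; Its capsule overlap sets or clears itself as the look-at actor in the top-down character's inventory system.
; On interact, it adds its item ID and quantity to that inventory and shows the NPC's quest widget even if adding fails.
; It destroys itself only when the add succeeds.
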(event OnComponentBeginOverlap(Capsule)
  (params (OverlappedComponent :type Primitive%20Component%20Object%20Reference) (OtherActor :type Actor%20Object%20Reference) (OtherComp :type Primitive%20Component%20Object%20Reference) (OtherBodyIndex :type Integer) (bFromSweep :type Boolean) (SweepResult :type Hit%20Result%20Structure%20%28by%20ref%29))
  (bind _asbp_top_down_character (Utilities|Casting|CastToBP_TopDownCharacter OtherActor))
  (Variables|/Game/TopDown/Blueprints/Inventory/BP_InventorySystem.BP_InventorySystem_C|SetLookAtActor (Variables|/Game/TopDown/Blueprints/BP_TopDownCharacter.BP_TopDownCharacter_C|GetBP_InventorySystem _asbp_top_down_character) self))

(event OnComponentEndOverlap(Capsule)
  (params (OverlappedComponent :type Primitive%20Component%20Object%20Reference) (OtherActor :type Actor%20Object%20Reference) (OtherComp :type Primitive%20Component%20Object%20Reference) (OtherBodyIndex :type Integer))
  (bind _asbp_top_down_character (Utilities|Casting|CastToBP_TopDownCharacter OtherActor))
  (Variables|/Game/TopDown/Blueprints/Inventory/BP_InventorySystem.BP_InventorySystem_C|SetLookAtActor (Variables|/Game/TopDown/Blueprints/BP_TopDownCharacter.BP_TopDownCharacter_C|GetBP_InventorySystem _asbp_top_down_character) 0))

(event EventBeginPlay)

(event Collision|EventActorBeginOverlap
  (params (OtherActor :type Actor%20Object%20Reference)))

(event EventTick
  (params (DeltaSeconds :type Float%20%28single-precision%29)))

(event EventInteractwith
  (params (PlayerCharacter :type BP%20Top%20Down%20Character%20Object%20Reference))
  (bind _bp_inventorysystem (Variables|/Game/TopDown/Blueprints/BP_TopDownCharacter.BP_TopDownCharacter_C|GetBP_InventorySystem PlayerCharacter))
  (Utilities|IsValid _bp_inventorysystem
    (:Is%20Valid
      (bind _success (Default|AddItemtoInventory _bp_inventorysystem (Variables|Default|GetItemID) (Variables|Default|GetQuantity)))
      (bind _returnvalue (Actor|GetActorOfClass "/Game/TopDown/Blueprints/Quest/NPC/4_NPCOldMan.4_NPCOldMan_C"))
      (Rendering|SetVisibility (Variables|/Game/TopDown/Blueprints/Quest/NameTag/BP_P_QuestAlert.BP_P_QuestAlert_C|GetQuest%20Widget _returnvalue) true false)
      (if _success
        (Actor|DestroyActor)))))

(fn ConstructionScript)

(fn InRangeOf
  (return ""))