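; BP_BlueCougar is an enemy that deals damage to the player through an attack hitbox.
; AttackCollision starts disabled on BeginPlay, and the OnAttackBegin and OnAttackEnd events switch it to query-only and back off.
; When the player character begins overlapping it, the cougar applies a fixed amount of damage, crediting its AI controller as instigator and itself as causer.
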(event OnComponentBeginOverlap(AttackCollision)
  (params (OverlappedComponent :type Primitive%20Component%20Object%20Reference) (OtherActor :type Actor%20Object%20Reference) (OtherComp :type Primitive%20Component%20Object%20Reference) (OtherBodyIndex :type Integer) (bFromSweep :type Boolean) (SweepResult :type Hit%20Result%20Structure%20%28by%20ref%29))
  (bind _returnvalue (Game|GetPlayerCharacter 0))
  (bind _self self)
  (if (== OtherActor _returnvalue)
    (Game|Damage|ApplyDamage _returnvalue 1.0 (AI|GetAIController _self) _self)))

(event Custom|OnAttackBegin
  (Collision|SetCollisionEnabled (Variables|Default|GetAttackCollision) "QueryOnly"))

(event Custom|OnAttackEnd
  (Collision|SetCollisionEnabled (Variables|Default|GetAttackCollision) "NoCollision"))

(event EventBeginPlay
  (Collision|SetCollisionEnabled (Variables|Default|GetAttackCollision) "NoCollision"))

(event Collision|EventActorBeginOverlap
  (params (OtherActor :type Actor%20Object%20Reference)))

(event EventTick
  (params (DeltaSeconds :type Float%20%28single-precision%29)))

(fn ConstructionScript)