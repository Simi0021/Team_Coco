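; AI controller for the cougar enemy that runs its behavior tree and reacts to seeing the player.
; On BeginPlay it starts BT_Cougar, sets a slow walk speed and writes the current state to the Blackboard.
; Perception updates go to HandleSightSense, which accepts only sight stimuli from the player character.
; Sighting sets TargetActor and raises the cougar to chase speed, while losing sight clears the target and restores the slow speed.
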(event OnTargetPerceptionUpdated(AIPerception)
  (params (Actor :type Actor%20Object%20Reference) (Stimulus :type AI%20Stimulus%20Structure))
  (CallFunction|HandleSightSense Actor Stimulus))

(event EventBeginPlay
  (AI|RunBehaviorTree "/Game/Enemy/Cougar/BT_Cougar.BT_Cougar")
  (bind _asbp_cougar (Utilities|Casting|CastToBP_Cougar (Pawn|GetControlledPawn)))
  (Variables|/Script/Engine.CharacterMovementComponent|SetMaxWalkSpeed (Variables|/Script/Engine.Character|GetCharacterMovement _asbp_cougar) 2e+02)
  (AI|Components|Blackboard|SetValueasEnum (Variables|Default|GetBlackboard) (Utilities|Name|MakeLiteralName "CurrentState") (Variables|Default|GetCurrentState)))

(event EventTick
  (params (DeltaSeconds :type Float%20%28single-precision%29)))

(fn ConstructionScript)

(fn HandleSightSense
  (params (Actor :type Actor%20Object%20Reference) (Stimulus :type AI%20Stimulus%20Structure))
  (bind _returnvalue (Class|AIPerceptionSystem|GetSenseClassforStimulus Stimulus))
  (if (== _returnvalue "/Script/AIModule.AISense_Sight")
    (if (== Actor (Game|GetPlayerCharacter 0))
      (AI|Components|Blackboard|SetValueasObject (Variables|Default|GetBlackboard) (Utilities|Name|MakeLiteralName "TargetActor") (Utilities|SelectObject (Game|GetPlayerCharacter 0) 0 (.bsuccessfullysensed Stimulus)))
      (if (.bsuccessfullysensed Stimulus)
        (bind _asbp_cougar (Utilities|Casting|CastToBP_Cougar (Pawn|GetControlledPawn)))
        (Variables|/Script/Engine.CharacterMovementComponent|SetMaxWalkSpeed (Variables|/Script/Engine.Character|GetCharacterMovement _asbp_cougar) 7.2e+02)
        (else
          (bind _asbp_cougar_2 (Utilities|Casting|CastToBP_Cougar (Pawn|GetControlledPawn)))
          (Variables|/Script/Engine.CharacterMovementComponent|SetMaxWalkSpeed (Variables|/Script/Engine.Character|GetCharacterMovement _asbp_cougar_2) 2e+02)))
      (else
        (return)))
    (else
      (return))))