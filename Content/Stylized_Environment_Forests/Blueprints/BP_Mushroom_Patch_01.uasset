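; A stylized forest mushroom patch Blueprint with two point lights that can be toggled on and off.
; A LightSwitch event uses a FlipFlop, enabling shadow casting and playing a timeline forward, or disabling shadows and reversing it.
; The timeline fades both lights' intensity between zero and a maximum through a Lerp.
; Tick, BeginPlay and the construction script are unused.
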(event Custom|LightSwitch
  (bind _pointlight1 (Variables|Default|GetPointLight1))
  (bind _pointlight (Variables|Default|GetPointLight))
  (Utilities|FlowControl|FlipFlop
    (:A
      (Rendering|Components|Light|SetCastShadows _pointlight true)
      (Rendering|Components|Light|SetCastShadows _pointlight1 true)
      (bind _intensity (Timeline|Timeline_0 PlayFromStart)
        (:Update
          (Rendering|Components|Light|SetIntensity (Variables|Default|GetPointLight) (Math|Float|Lerp 0.0 1.9e+03 _intensity))
          (Rendering|Components|Light|SetIntensity (Variables|Default|GetPointLight1) (Math|Float|Lerp 0.0 1.9e+03 _intensity)))))
    (:B
      (Rendering|Components|Light|SetCastShadows _pointlight false)
      (Rendering|Components|Light|SetCastShadows _pointlight1 false)
      (Timeline|Timeline_0 ReverseFromEnd))))

(event EventBeginPlay)

(event Collision|EventActorBeginOverlap
  (params (OtherActor :type Actor%20Object%20Reference)))

(event EventTick
  (params (DeltaSeconds :type Float%20%28single-precision%29)))

(fn ConstructionScript)